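; BP_TimelineActor is an actor that slides its Sphere component back and forth along relative X, with toggleable playback.
; PreesP switches between PlayTimelineActor and StopTimelineActor based on IsPlay.
; A timeline's value, scaled to a distance, sets the sphere's location on each update.
; When the timeline finishes, IsMoveRight flips and execution loops back to choose Play or Reverse, creating a ping-pong motion.
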(event Custom|PlayTimelineActor
  (Variables|Default|SetIsPlay true)
  (if (Variables|Default|GetIsMoveRight) :!label _label
    (bind _value (Timeline|타임라인_0 Play)
      (:Update
        (Transformation|SetRelativeLocation (Variables|Default|GetSphere) (Math|Vector|MakeVector (* _value 3e+02) 0.0 0.0) false false))
      (:Finished
        (Variables|Default|SetIsMoveRight (not (Variables|Default|GetIsMoveRight)))
        (goto _label)))
    (else
      (Timeline|타임라인_0 Reverse))))

(event Custom|StopTimelineActor
  (Variables|Default|SetIsPlay false)
  (bind _value (Timeline|타임라인_0 Stop)
    (:Update
      (Transformation|SetRelativeLocation (Variables|Default|GetSphere) (Math|Vector|MakeVector (* _value 3e+02) 0.0 0.0) false false))
    (:Finished
      (Variables|Default|SetIsMoveRight (not (Variables|Default|GetIsMoveRight)))
      (if (Variables|Default|GetIsMoveRight)
        (Timeline|타임라인_0 Play)
        (else
          (Timeline|타임라인_0 Reverse))))))

(event Custom|PreesP
  (if (Variables|Default|GetIsPlay)
    (CallFunction|StopTimelineActor)
    (else
      (CallFunction|PlayTimelineActor))))

(event EventBeginPlay)

(fn ConstructionScript)