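; BP_MyPawn2 is a player pawn that flies freely along the camera's forward and right vectors, with controller look input and an adjustable, clamped move speed.
; On BeginPlay it gathers all BP_TimelineActor and BP_RotationBall actors into one Actors array.
; Pressing P loops that array and casts each entry to call PressP on timeline actors or PressP2 on rotation balls.
; Movement uses unswept world offsets scaled by speed without delta time.
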(event EventBeginPlay
  (Utilities|FlowControl|Sequence
    (:then_0
      (bind _outactors (Actor|GetAllActorsOfClass "/Game/BP_TimelineActor.BP_TimelineActor_C"))
      (for _array_element _outactors
        (Utilities|Array|Add (Variables|Default|GetActors) _array_element)))
    (:then_1
      (bind _outactors_2 (Actor|GetAllActorsOfClass "/Game/BP_RotationBall.BP_RotationBall_C"))
      (for _array_element_2 _outactors_2
        (Utilities|Array|Add (Variables|Default|GetActors) _array_element_2)))))

(event Input|ActionEvents|InputActionSpeedUp
  (params (Key :type Key%20Structure :default "None"))
  ;[1 1 1] 이동 속도 변경 코드
  (:Pressed
    (bind _output_get (Variables|Default|SetPlayerSpeed (+ (Variables|Default|GetPlayerSpeed) 1e+01)))
    (if (>= _output_get 1e+02)
      (Variables|Default|SetPlayerSpeed 1e+02))))

(event Input|ActionEvents|InputActionSpeedDown
  (params (Key :type Key%20Structure :default "None"))
  ;[1 1 1] 이동 속도 변경 코드
  (:Pressed
    (bind _output_get (Variables|Default|SetPlayerSpeed (- (Variables|Default|GetPlayerSpeed) 1e+01)))
    (if (<= _output_get 1e+01)
      (Variables|Default|SetPlayerSpeed 1e+01))))

(event Input|AxisEvents|InputAxisMoveForward
  (params (AxisValue :type Float%20%28single-precision%29))
  ;[1 1 1] 이동 처리 코드
  (Transformation|AddActorWorldOffset (* (Transformation|GetActorForwardVector (Game|GetPlayerCameraManager 0)) (* AxisValue (Variables|Default|GetPlayerSpeed)))))

(event Input|AxisEvents|InputAxisMoveRight
  (params (AxisValue :type Float%20%28single-precision%29))
  ;[1 1 1] 이동 처리 코드
  (Transformation|AddActorWorldOffset (* (Transformation|GetActorRightVector (Game|GetPlayerCameraManager 0)) (* AxisValue (Variables|Default|GetPlayerSpeed)))))

(event Input|AxisEvents|InputAxisLookUp
  (params (AxisValue :type Float%20%28single-precision%29))
  ;[1 1 1] 이동 처리 코드
  (Pawn|Input|AddControllerPitchInput AxisValue))

(event Input|AxisEvents|InputAxisLookRight
  (params (AxisValue :type Float%20%28single-precision%29))
  ;[1 1 1] 이동 처리 코드
  (Pawn|Input|AddControllerYawInput AxisValue))

(event Input|KeyboardEvents|P
  (params (Key :type Key%20Structure :default "None"))
  (:Pressed
    (for _array_element (Variables|Default|GetActors)
      (bind _asbp_timeline_actor (Utilities|Casting|CastToBP_TimelineActor _array_element)
        (:then
          (Default|PressP _asbp_timeline_actor))
        (:CastFailed
          (bind _asbp_rotation_ball (Utilities|Casting|CastToBP_RotationBall _array_element))
          (Default|PressP2 _asbp_rotation_ball))))))

(fn ConstructionScript)